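; BP_RockPlanter is a pickup item that the third-person character can carry in its hand.
; On overlap it caches the character and passes itself to that character's PickUpItem.
; PickUp attaches it to the player mesh's hand_r socket, while Drop destroys the actor rather than releasing it.
; PlantSeed is empty, and the logic that would spawn a BP_Tree at the planter's transform is disconnected.
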(event `self.ReceiveActorBeginOverlap`
  (params (OtherActor :type "Actor Object Reference"))
  (bind _asbp_third_person_character (cast `/Game/ThirdPerson/Blueprints/BP_ThirdPersonCharacter` OtherActor))
  (set `self.Player` _asbp_third_person_character) ; Promote To Variable
  (`/Game/ThirdPerson/Blueprints/BP_ThirdPersonCharacter.PickUpItem` _asbp_third_person_character self))

(event `/Game/Blueprints/I_SeedPlanter.PickUp`
  (`KismetSystemLibrary.PrintText` "This rock planter has been picked up")
  (`self.K2_AttachToComponent` (`Character.Mesh` (`self.Player`)) "hand_r" "SnapToTarget" "SnapToTarget" "KeepRelative"))

(event `/Game/Blueprints/I_SeedPlanter.PlantSeed`)

(event `/Game/Blueprints/I_SeedPlanter.Drop`
  (`KismetSystemLibrary.PrintText` "Trying to drop the planter")
  (`self.K2_DestroyActor`))

(fn `UserConstructionScript`)