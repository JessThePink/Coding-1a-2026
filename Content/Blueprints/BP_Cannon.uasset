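; Cannon actor that spawns and launches a BP_CannonBall shortly after BeginPlay (marked as testing) and whenever an actor overlaps it.
; Each shot spawns the ball at the BoxSpawnPoint transform, then pushes its Cube along that cube's forward vector with a mass-independent AddForce.
; The LaunchCannonBall event only prints debug text; the spawn and force logic follows its call in the shared firing chain.
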(event `self.ReceiveBeginPlay`
  (`KismetSystemLibrary.Delay` 0.2) ; Testing
  (`self.LaunchCannonBall` :!label _label)
  (bind _returnvalue (`|SpawnActorFromClass` "/Game/Blueprints/BP_CannonBall.BP_CannonBall_C" (`SceneComponent.K2_GetComponentToWorld` (`self.BoxSpawnPoint`)) "Undefined" "MultiplyWithRoot" null null))
  (bind _cube (`/Game/Blueprints/BP_CannonBall.Cube` _returnvalue))
  (`PrimitiveComponent.AddForce` _cube (* (`SceneComponent.GetForwardVector` _cube) 100000.0) "None" true))

(event `self.ReceiveActorBeginOverlap`
  (params (OtherActor :type "Actor Object Reference"))
  (goto _label))

(event `LaunchCannonBall`
  (`KismetSystemLibrary.PrintText` "Wabam"))

(fn `UserConstructionScript`)