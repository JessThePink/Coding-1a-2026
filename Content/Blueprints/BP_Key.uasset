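; BP_Key is a collectible key pickup shown with a prototype coin mesh.
; On BeginPlay, two timelines hand off to each other in an endless loop, one forward and one in reverse, to animate the mesh's relative location.
; When a BP_ThirdPersonCharacter overlaps it, the pickup increments that character's TotalKeys, prints a "Coin Collected!" message and destroys itself.
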(event `self.ReceiveBeginPlay`
  (bind (_direction _newtrack_0) (`Timeline|MovingCoin` :!label _label)
    (:`Update`
      (`SceneComponent.K2_SetRelativeLocation` (`self.SM_PolygonPrototype_Icon_Coin_01`) _newtrack_0 false false))
    (:`Finished`
      (bind (_direction_2 _newtrack_0_2) (`Timeline|Timeline` :!via `ReverseFromEnd`)
        (:`Update`
          (`SceneComponent.K2_SetRelativeLocation` (`self.SM_PolygonPrototype_Icon_Coin_01`) _newtrack_0_2 false false))
        (:`Finished`
          (goto _label :!via `PlayFromStart`))))))

(event `self.ReceiveActorBeginOverlap`
  (params (OtherActor :type "Actor Object Reference"))
  (bind _asbp_third_person_character (cast `/Game/ThirdPerson/Blueprints/BP_ThirdPersonCharacter` OtherActor))
  (`/Engine/EditorBlueprintResources/StandardMacros.IncrementInt` (`/Game/ThirdPerson/Blueprints/BP_ThirdPersonCharacter.TotalKeys` _asbp_third_person_character)
    (:`  `
      (`KismetSystemLibrary.PrintText` "Coin Collected!")
      (`self.K2_DestroyActor`))))

(fn `UserConstructionScript`)