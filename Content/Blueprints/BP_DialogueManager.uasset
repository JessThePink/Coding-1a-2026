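; BP_DialogueManager is a dialogue Blueprint meant to show lines from a Dialogue array one at a time.
; Its DisplayNextLine event is empty, and the display logic is left unwired, so it never runs.
; That disconnected chain wraps Index to the start past the last line, prints the current entry with Print Text as a timed debug message, then increments Index.
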(event `DisplayNextLine`)

(fn `UserConstructionScript`)