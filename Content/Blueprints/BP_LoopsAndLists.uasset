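; BP_LoopsAndLists is a Blueprint that demonstrates while loops, array iteration and delayed self-calls.
; On BeginPlay, a delayed while loop counts WhileCounter down, printing each number in a color cycled from Colors by modulo 7.
; In parallel, MakeCoinsJump starts after a shorter delay, raises every BP_Key actor, prints how many moved, then calls itself again each second indefinitely.
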(event `self.ReceiveBeginPlay`
  (bind _whilecounter (`self.WhileCounter`))
  (`|ExecutionSequence`
    (:`then_0`
      (`KismetSystemLibrary.Delay` 2.0)
      (while (> _whilecounter 0)
        (`KismetSystemLibrary.PrintText` (`|FormatText` "We are in loop number {count}" _whilecounter) true true (`|GetArrayItem` (`self.Colors`) (mod (`self.WhileCounter`) 7)) 22.0)
        (`/Engine/EditorBlueprintResources/StandardMacros.DecrementInt` (`self.WhileCounter`))))
    (:`then_1`
      (`KismetSystemLibrary.Delay` 1.0)
      (`self.MakeCoinsJump`))))

(event `MakeCoinsJump`
  (bind _outactors (`GameplayStatics.GetAllActorsOfClass` "/Game/Blueprints/BP_Key.BP_Key_C"))
  (for _array_element _outactors
    (`SceneComponent.K2_AddRelativeLocation` (`/Game/Blueprints/BP_Key.DefaultSceneRoot` _array_element) (0.0 0.0 50.0) false false))
  (`KismetSystemLibrary.PrintText` (`|FormatText` "We have raised {count} keys." (`KismetArrayLibrary.Array_Length` _outactors)) true true (struct :`G` 0.66 :`B` 1.0 :`A` 1.0) 22.0)
  (`KismetSystemLibrary.Delay` 1.0)
  (`self.MakeCoinsJump`) ; the function calls itself\none second after completion
)

(fn `UserConstructionScript`)